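; Drone body pawn that spins its two fan meshes and hooks itself up to its AI on spawn.
; Every tick, both fans rotate around local yaw at a frame-rate-independent speed.
; On BeginPlay it casts its controller to DroneAI, starts the DroneAIBB blackboard and registers itself under the DroneActor key.
; It also stores its start location and a reference to the player character.
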(event Custom|RotateFan
  (for _array_element (Utilities|Array|MakeArray (Variables|Default|GetFan1) (Variables|Default|GetFan2))
    (Utilities|IsValid (Variables|/Script/Engine.StaticMeshComponent|GetStaticMesh _array_element)
      (:Is%20Valid
        (Transformation|AddLocalRotation _array_element (Math|Rotator|MakeRotator 0.0 0.0 (* (Utilities|Time|GetWorldDeltaSeconds) 1000)) false false)))))

(event EventBeginPlay
  (Utilities|FlowControl|Sequence
    (:then_0
      (bind _asdrone_ai (Utilities|Casting|CastToDroneAI (Pawn|GetController)))
      (bind _output_get (Variables|Default|SetAs%20Drone%20AI _asdrone_ai))
      (bind _blackboardcomponent (Class|AIController|UseBlackboard _output_get "/Game/Mesh/Drone/blueprint/AIControl/DroneAI-BB.DroneAI-BB"))
      (bind _output_get_2 (Variables|Default|SetBlackboardComponent-Ref _blackboardcomponent))
      (AI|Components|Blackboard|SetValueasObject _output_get_2 (Utilities|Name|MakeLiteralName "DroneActor") self))
    (:then_1
      (Variables|Default|SetStartLocation (Transformation|GetActorLocation)))
    (:then_2
      (bind _asplayer_character (Utilities|Casting|CastToPlayerCharacter (Game|GetPlayerCharacter 0)))
      (Variables|Default|SetPlayerRef _asplayer_character))))

(event EventTick
  (params (DeltaSeconds :type Float%20%28single-precision%29))
  (Utilities|FlowControl|Sequence
    (:then_0
      (CallFunction|RotateFan))))

(fn ConstructionScript)